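; Blueprint function library for UI that formats a float number of seconds as a clock-style time string.
; Both functions break the value into a timespan and zero-pad minutes and seconds, leaving out hours.
; The Normal variant returns minutes:seconds, while Verbose appends the first two characters of the unpadded milliseconds value.
; Both graphs also contain unused leftover formatting chains.
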(fn ConvertFloattoTimeVerbose
  (params (Seconds :type Float%20%28single-precision%29))
  (bind _returnvalue (Math|Timespan|FromSeconds Seconds))
  (bind (_days _hours _minutes _seconds _milliseconds) (Math|Timespan|BreakTimespan _returnvalue))
  (bind _returnvalue_2 (Utilities|String|ToString(Integer) _seconds))
  (bind _returnvalue_3 (Utilities|String|ToString(Integer) _minutes))
  (return (Utilities|String|Append (select (> _minutes 9) _returnvalue_3 (Utilities|String|Append "0" _returnvalue_3)) " : " (select (> _seconds 9) _returnvalue_2 (Utilities|String|Append "0" _returnvalue_2)) " : " (Utilities|String|Left (Utilities|String|ToString(Integer) _milliseconds) 2))))

(fn ConvertFloattoTimeNormal
  (params (Seconds :type Float%20%28single-precision%29))
  (bind _returnvalue (Math|Timespan|FromSeconds Seconds))
  (bind (_days _hours _minutes _seconds _milliseconds) (Math|Timespan|BreakTimespan _returnvalue))
  (bind _returnvalue_2 (Utilities|String|ToString(Integer) _seconds))
  (bind _returnvalue_3 (Utilities|String|ToString(Integer) _minutes))
  (return (Utilities|String|Append (select (> _minutes 9) _returnvalue_3 (Utilities|String|Append "0" _returnvalue_3)) " : " (select (> _seconds 9) _returnvalue_2 (Utilities|String|Append "0" _returnvalue_2)))))