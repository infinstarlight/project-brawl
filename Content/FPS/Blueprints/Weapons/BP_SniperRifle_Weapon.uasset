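; Sniper rifle weapon Blueprint with breath-hold steadying, scope overlay and stepped zoom.
; StopHoldBreath saves the timer's remaining breath, restarts the breathing camera shake and starts a looping timer that refills breath up to its maximum.
; Scope toggling, shot shake, breath-hold start and zoom steps that halve or double aiming FOV sit in chains with no connected trigger, so they never run.
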(event Custom|RegenBreath
  (bind _maxbreathleft_0 (Variables|Default|GetMaxBreathLeft_0))
  ;[1 1 1] Hold Breath System
  (if (> (+ (Variables|Default|GetBreathLeft_0) 0.15) _maxbreathleft_0)
    (Variables|Default|SetBreathLeft_0 _maxbreathleft_0)
    (Utilities|Time|ClearandInvalidateTimerbyHandle (Variables|Default|GetRegenBreathTimerHandle_0))
    (else
      (Variables|Default|SetBreathLeft_0 (+ (Variables|Default|GetBreathLeft_0) 0.15)))))

(event EventBeginPlay
  (|CallParentFunction) ; This node is disabled and will not be called.\nDrag off pins to build functionality.
)

(event Collision|EventActorBeginOverlap
  (params (OtherActor :type Actor%20Object%20Reference)))

(event EventStopHoldBreath
  (bind _holdbreathtimer_0 (Variables|Default|GetHoldBreathTimer_0))
  ;[1 1 1] Hold Breath System
  (if (Utilities|Time|IsTimerActivebyHandle _holdbreathtimer_0)
    (Variables|Default|SetBreathLeft_0 (Utilities|Time|GetTimerRemainingTimebyHandle _holdbreathtimer_0))
    (bind _returnvalue (Utilities|Time|SetTimerbyEvent (delegate Custom|RegenBreath) 0.5 true))
    (Variables|Default|SetRegenBreathTimerHandle_0 _returnvalue)
    (Utilities|IsValid (Variables|Default|GetBreathingShakeRef)
      (:Is%20Not%20Valid
        (bind _returnvalue_2 (Class|PlayerCameraManager|PlayCameraShake (Game|GetPlayerCameraManager 0) "/Game/FPS/Blueprints/CameraShake/BreathingShake.BreathingShake_C" 1.0 "CameraLocal" "0, 0, 0"))
        (Variables|Default|SetBreathingShakeRef _returnvalue_2)
        (Utilities|Time|ClearandInvalidateTimerbyHandle (Variables|Default|GetHoldBreathTimer_0))))))

(fn ConstructionScript
  (|CallParentFunction))