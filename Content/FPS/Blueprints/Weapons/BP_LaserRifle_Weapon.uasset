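; Laser rifle weapon Blueprint for the FPS game, with scope zoom and a camera shake on firing.
; Begin aiming defers to the parent, while end aiming restores visibility, hides the scope on the player controller's gameplay widget and stops all camera shakes.
; Scope zoom input passes through to ZoomScope, and the shot shake event plays the sniper shake on the first player's camera manager.
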(event EventBeginPlay
  (|CallParentFunction) ; This node is disabled and will not be called.\nDrag off pins to build functionality.
)

(event EventScopeZoom
  (params (Up :type Boolean))
  (CallFunction|ZoomScope Up))

(event EventOnBeginAiming
  ;[1 1 1] On Begin Amining
  (|CallParentFunction))

(event EventOnEndAiming
  ;[1 1 1] On End Aiming
  (CallFunction|ToggleVisibility true)
  (bind _asbase_character_pc (Utilities|Casting|CastToBaseCharacterPC (Game|GetPlayerController 0)))
  (Default|SetScopeVisibility (Variables|/Game/FPS/Blueprints/PlayerController/BaseCharacterPC.BaseCharacterPC_C|GetGameplayWB _asbase_character_pc) false)
  (CameraShake|StopAllCameraShakes (Game|GetPlayerCameraManager 0) true))

(event EventPlayShotShake
  ;[1 1 1] Shot Shake
  (Class|PlayerCameraManager|PlayCameraShake (Game|GetPlayerCameraManager 0) "/Game/FPS/Blueprints/CameraShake/SniperShake.SniperShake_C" 1.0 "CameraLocal" "0, 0, 0"))

(fn ConstructionScript
  (|CallParentFunction))