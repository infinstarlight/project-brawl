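; BP_Rocket is a rocket projectile that builds on inherited grenade logic and explodes on impact.
; BeginPlay runs the parent logic, then nudges StartLocation along X.
; Hit zeroes TimeToExplode and calls ServerExplodeGrenade unless the hit actor is player pawn 0, a check against that index rather than the owner.
; Unconnected leftover nodes hold a line-trace, HealthComponent and owner check that never runs.
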(event EventBeginPlay
  (|CallParentFunction)
  (Variables|Default|SetStartLocation (+ (Variables|Default|GetStartLocation) "50.000000, 0, 0")))

(event Collision|EventActorBeginOverlap
  (params (OtherActor :type Actor%20Object%20Reference)))

(event EventTick
  (params (DeltaSeconds :type Float%20%28single-precision%29)))

(event Collision|EventHit
  (params (MyComp :type Primitive%20Component%20Object%20Reference) (Other :type Actor%20Object%20Reference) (OtherComp :type Primitive%20Component%20Object%20Reference) (bSelfMoved :type Boolean) (HitLocation :type Vector :default "0, 0, 0") (HitNormal :type Vector :default "0, 0, 0") (NormalImpulse :type Vector :default "0, 0, 0") (Hit :type Hit%20Result%20Structure%20%28by%20ref%29))
  (Variables|Default|SetTimeToExplode 0.0)
  (if (!= (.HitActor (Collision|BreakHitResult Hit)) (Game|Player|GetPlayerPawn 0))
    (CallFunction|ServerExplodeGrenade)))

(fn ConstructionScript
  (|CallParentFunction))