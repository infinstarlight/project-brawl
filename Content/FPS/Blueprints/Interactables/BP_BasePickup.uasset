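; Base pickup actor for an FPS, providing shared helpers for health recovery and weapon pickups.
; RecoverPlayerHealth routes healing through ApplyDamage with a transformed amount and plays a sound; AddNewWeapon passes a weapon class to BP_BaseCharacter.
; Both mark the pickup used and call HidePickup, which starts a ReactivateDelay timer and sets the box to query-only and particles visible.
; OnInteracted disables box collision and hides the particles.
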(event Custom|OnInteracted
  (Collision|SetCollisionEnabled (Variables|Default|GetBox) "NoCollision")
  (Rendering|SetVisibility (Variables|Default|GetParticleSystem) false false))

(event EventBeginPlay)

(event Collision|EventActorBeginOverlap
  (params (OtherActor :type Actor%20Object%20Reference)))

(event EventTick
  (params (DeltaSeconds :type Float%20%28single-precision%29)))

(fn ConstructionScript)

(fn RecoverPlayerHealth
  (params (DamagedActor :type Actor%20Object%20Reference) (BaseDamage :type Float%20%28single-precision%29))
  (bind _result (Math|Float|NegateFloat BaseDamage)
    (:%20%20
      (Game|Damage|ApplyDamage DamagedActor _result 0 self)
      (Variables|Default|SetbHasBeenUsed? true)
      (Audio|PlaySound2D 0 1.0 1.0 0.0 0 0)
      (CallFunction|HidePickup))))

(fn AddNewWeapon
  (params (OtherActor :type Actor%20Object%20Reference) (NewWeaponClass :type BP%20Base%20Weapon%20Class%20Reference%20%28by%20ref%29))
  (Utilities|IsValid OtherActor
    (:Is%20Valid
      (Default|PickupNewWeapon (.AsBP%20Base%20Character (Utilities|Casting|CastToBP_BaseCharacter OtherActor)) NewWeaponClass)
      (Variables|Default|SetbHasBeenUsed? true)
      (CallFunction|HidePickup))))

(fn HidePickup
  (if (Variables|Default|GetbHasBeenUsed?)
    (Utilities|Time|SetTimerbyEvent (EventDispatchers|CreateEvent :!event Custom|OnInteracted) (Variables|Default|GetReactivateDelay))
    (Collision|SetCollisionEnabled (Variables|Default|GetBox) "QueryOnly")
    (Rendering|SetVisibility (Variables|Default|GetParticleSystem) true false)))