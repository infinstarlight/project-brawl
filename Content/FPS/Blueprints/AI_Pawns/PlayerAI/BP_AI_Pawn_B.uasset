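; AI pawn variant B for the FPS game, a child Blueprint that defines the bot's weapon loadout.
; On BotEquipWeapon, if no valid current weapon exists, it equips the mech assault rifle as primary and a second weapon as secondary, both with initial values.
; It then makes the primary the current weapon and hides the secondary.
; The construction script only calls the parent, and the other events are disabled or empty.
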(event EventBeginPlay
  (|CallParentFunction) ; This node is disabled and will not be called.\nDrag off pins to build functionality.
)

(event Collision|EventActorBeginOverlap
  (params (OtherActor :type Actor%20Object%20Reference)))

(event EventTick
  (params (DeltaSeconds :type Float%20%28single-precision%29))
  (|CallParentFunction DeltaSeconds) ; This node is disabled and will not be called.\nDrag off pins to build functionality.
)

(event EventBotEquipWeapon
  (Utilities|IsValid (Variables|Default|GetCurrentWeapon)
    (:Is%20Not%20Valid
      (bind _output_get (Variables|Default|SetPrimaryWeaponToSpawn "/Game/FPS/Blueprints/Weapons/BP_AssaultRifle_Weapon_Mech.BP_AssaultRifle_Weapon_Mech_C"))
      (CallFunction|EquipWeapon _output_get 0 true)
      (CallFunction|EquipWeapon "/Game/FPS/Blueprints/Weapons/BP_SecondaryWeapon_02.BP_SecondaryWeapon_02_C" 0 true)
      (Variables|Default|SetCurrentWeapon (Variables|Default|GetPrimaryWeapon))
      (CallFunction|SetWeaponVisibility (Variables|Default|GetSecondaryWeapon) true))))

(fn ConstructionScript
  (|CallParentFunction))