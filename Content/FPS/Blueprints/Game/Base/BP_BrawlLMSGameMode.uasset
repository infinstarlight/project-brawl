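; BP_BrawlLMSGameMode is the game mode for the LMS (likely Last Man Standing) brawl match type in the FPS game.
; On BeginPlay it gathers player spawn points, checks game options, manages the bot count, then sets the game type to LMS and enables friendly fire.
; On the server, each valid new player is added to the controller list and given a zero-point score entry.
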(event EventBeginPlay
  (CallFunction|GetPlayerSpawnPoints)
  (CallFunction|CheckGameOptions)
  (CallFunction|ManageNumberOfBots)
  (Variables|Default|SetCurrentGameType "LMS")
  (Variables|Default|SetbEnableFriendlyFire true))

(event EventTick
  (params (DeltaSeconds :type Float%20%28single-precision%29))
  (|CallParentFunction DeltaSeconds) ; This node is disabled and will not be called.\nDrag off pins to build functionality.
)

(event EventHandleStartingNewPlayer
  (params (NewPlayer :type Player%20Controller%20Object%20Reference))
  (Networking|SwitchHasAuthority
    (:Authority
      (Utilities|IsValid NewPlayer
        (:Is%20Valid
          (Utilities|Array|Add (Variables|Default|GetCurrentPlayerControllers) NewPlayer)
          (Utilities|Array|AddUnique (Variables|Default|GetAllPlayerPoints) (Utilities|Struct|MakePlayerPoints 0 0)))))))

(event EventOnLogout
  (params (ExitingController :type Controller%20Object%20Reference))
  (|CallParentFunction ExitingController))

(fn ConstructionScript
  (|CallParentFunction))