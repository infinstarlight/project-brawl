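; Base flag actor for capture-the-flag that handles pickup, return and capture scoring.
; On server-side capsule overlap while untaken, a living character not on FlagTakerTeam picks it up, attaching it to the mesh's FlagSocket.
; A FlagTakerTeam character resets it to its BeginPlay location.
; Before that reset, if they carry a flag and this one is near home, TryToAddPoint awards team and player points and resets the carried flag.
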(event OnComponentBeginOverlap(Capsule)
  (params (OverlappedComponent :type Primitive%20Component%20Object%20Reference) (OtherActor :type Actor%20Object%20Reference) (OtherComp :type Primitive%20Component%20Object%20Reference) (OtherBodyIndex :type Integer) (bFromSweep :type Boolean) (SweepResult :type Hit%20Result%20Structure%20%28by%20ref%29))
  ;[0.01562 0.01562 0.01562] OnOverlap with flag capsule
  (Networking|SwitchHasAuthority
    (:Authority
      (if (not (Variables|Default|GetbFlagTaken))
        (bind _asbp_base_character (Utilities|Casting|CastToBP_BaseCharacter OtherActor))
        (bind _output_get (Variables|Default|SetPawnRef _asbp_base_character))
        (if (not (Variables|/Game/FPS/Blueprints/CharacterAndClasses/BP_BaseCharacter.BP_BaseCharacter_C|GetbDead _output_get))
          (if (not (Utilities|Enum|Equal(Enum) (Variables|/Game/FPS/Blueprints/CharacterAndClasses/BP_BaseCharacter.BP_BaseCharacter_C|GetPawnTeam _asbp_base_character) (Variables|Default|GetFlagTakerTeam)))
            (if (not (Variables|/Game/FPS/Blueprints/CharacterAndClasses/BP_BaseCharacter.BP_BaseCharacter_C|GetbCarringFlag (Variables|Default|GetPawnRef)))
              (Default|OnPickupFlag (Variables|Default|GetPawnRef) self)
              (Variables|Default|SetbFlagTaken true)
              (Utilities|IsValid (Variables|Default|GetPawnRef)
                (:Is%20Valid
                  (Transformation|AttachComponentToComponent (Variables|/Script/Engine.Character|GetMesh (Variables|Default|GetPawnRef)) "FlagSocket" "SnapToTarget" "KeepRelative" "KeepRelative" true))))
            (else
              ;;[1 1 1] Your Team flag
              (CallFunction|TrytoAddPoint)
              (Transformation|Teleport (Variables|Default|GetInitialPossition) (Variables|Default|GetInitialRotation))
              (Transformation|SetActorRotation "0, 0, 0")
              (Utilities|FlowControl|Delay 0.2)
              (Utilities|IsValid (Variables|Default|GetPawnRef)
                (:Is%20Valid
                  (Default|OnDropFlag (Variables|Default|GetPawnRef)))
                (:Is%20Not%20Valid
                  _))
              (Variables|Default|SetbFlagTaken false))))))))

(event EventBeginPlay
  ;[1 0.2273 0.1175] BeginPlay
  (Variables|Default|SetInitialPossition (Transformation|GetActorLocation))
  (Variables|Default|SetInitialRotation (Transformation|GetActorRotation)))

(fn ConstructionScript)

(fn TrytoAddPoint
  (bind _pawnref (Variables|Default|GetPawnRef))
  (bind _pawnref_2 (Variables|Default|GetPawnRef))
  (bind _flagref (Variables|/Game/FPS/Blueprints/CharacterAndClasses/BP_BaseCharacter.BP_BaseCharacter_C|GetFlagRef _pawnref))
  (if (and (Variables|/Game/FPS/Blueprints/CharacterAndClasses/BP_BaseCharacter.BP_BaseCharacter_C|GetbCarringFlag (Variables|Default|GetPawnRef)) (Math|Vector|Equal(Vector) (Variables|Default|GetInitialPossition) (Transformation|GetActorLocation) 5e+01))
    ;[1 1 1] Add points
    (bind _asfps_ctf_gs (Utilities|Casting|CastToFPS_CTF_GS (Game|GetGameState)))
    (Default|AddTeamPoints _asfps_ctf_gs (Variables|/Game/FPS/Blueprints/CharacterAndClasses/BP_BaseCharacter.BP_BaseCharacter_C|GetbPawnTeam _pawnref_2))
    (bind _asfps_player_state (Utilities|Casting|CastToFPS_PlayerState (Variables|/Script/Engine.Pawn|GetPlayerState _pawnref_2)))
    (Default|AddScorePoints _asfps_player_state 3.5e+02 "FLAG CAPTURED")
    ;[1 1 1] ResetFlag
    (Default|DropFlag _pawnref)
    (Transformation|SetActorLocation _flagref (Variables|BP_BaseFlag_C|GetInitialPossition _flagref) false true)))